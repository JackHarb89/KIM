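; Player character Blueprint that relays icon changes and an eye-UI toggle to the KIMHUD_BP HUD of player 0.
; SwitchIconState passes its Type straight through to the HUD.
; Pressing E casts the HUD's EyeUI to the EysOpening widget and calls ToggleAnimation on it.
; BeginPlay, overlap, Tick and the construction script are empty.
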(event EventBeginPlay)

(event EventActorBeginOverlap
  (params (OtherActor :type Actor%20Object%20Reference)))

(event EventSwitchIconState
  (params (Type :type EKIMInteractionTypes%20Enum :default "NONE"))
  (bind _askimhud_bp (Utilities|Casting|CastToKIMHUD_BP (HUD|GetHUD (Game|GetPlayerController 0))))
  (Default|SwitchIconState _askimhud_bp Type))

(event EventTick
  (params (DeltaSeconds :type Float%20%28single-precision%29)))

(event Input|KeyboardEvents|E
  (params (Key :type Key%20Structure :default "AnyKey"))
  (:Pressed
    (bind _askimhud_bp (Utilities|Casting|CastToKIMHUD_BP (HUD|GetHUD (Game|GetPlayerController 0))))
    (bind _aseys_opening (Utilities|Casting|CastToEysOpening (Variables|/Game/Blueprint/UI/KIMHUD_BP.KIMHUD_BP_C|GetEyeUI _askimhud_bp)))
    (Default|ToggleAnimation _aseys_opening)))

(fn ConstructionScript)