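; Fire indicator actor that shows fire spreading outward across a bounded hex grid from its own location.
; Ignite seeds the origin; every TimeToIgnition, Tick expands the frontier to six neighbors, breadth-first.
; SpawnInstance rejects out-of-bounds or already recorded positions, then adds instanced hexagon and raised, double-scale fire symbol meshes.
; Tick also spins every fire symbol by updating its instance yaw each frame.
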(event Custom|Ignite
  (bind _returnvalue (Transformation|GetActorLocation))
  (bind _returnvalue_2 (Transformation|GetActorTransform))
  (bind (_x _y _z) (Math|Vector|BreakVector _returnvalue))
  (bind (_location _rotation _scale) (Math|Transform|BreakTransform _returnvalue_2))
  (Utilities|Array|Add (Variables|Default|GetPositionsToExpand) _returnvalue)
  (Utilities|Array|Add (Variables|Default|GetTotalPositions) _returnvalue)
  (Class|InstancedStaticMeshComponent|AddInstanceWorldSpace (Variables|Default|GetHexagons) (Transformation|GetActorTransform))
  (Class|InstancedStaticMeshComponent|AddInstanceWorldSpace (Variables|Default|GetFireSymbole) (Math|Transform|MakeTransform (Math|Vector|MakeVector _x _y (+ _z 25.0)) _rotation (* _scale 2))))

(event EventTick
  (params (DeltaSeconds :type Float%20%28single-precision%29))
  (bind _firesymbole (Variables|Default|GetFireSymbole))
  (Utilities|FlowControl|Sequence
    (:then_0
      (for _index (range 0 (Components|InstancedStaticMesh|GetInstanceCount _firesymbole))
        (Components|InstancedStaticMesh|UpdateInstanceTransform _firesymbole _index (Math|Transform|MakeTransform (.Location (Math|Transform|BreakTransform (.OutInstanceTransform (Components|InstancedStaticMesh|GetInstanceTransform _firesymbole _index true)))) (Math|Rotator|MakeRotator (.Roll (Math|Rotator|BreakRotator (.Rotation (Math|Transform|BreakTransform (.OutInstanceTransform (Components|InstancedStaticMesh|GetInstanceTransform _firesymbole _index true)))))) (.Pitch (Math|Rotator|BreakRotator (.Rotation (Math|Transform|BreakTransform (.OutInstanceTransform (Components|InstancedStaticMesh|GetInstanceTransform _firesymbole _index true)))))) (+ (.Yaw (Math|Rotator|BreakRotator (.Rotation (Math|Transform|BreakTransform (.OutInstanceTransform (Components|InstancedStaticMesh|GetInstanceTransform _firesymbole _index true)))))) 1.0)) (.Scale (Math|Transform|BreakTransform (.OutInstanceTransform (Components|InstancedStaticMesh|GetInstanceTransform _firesymbole _index true))))) true true)))
    (:then_1
      (bind _output_get (Variables|Default|SetTimer (+ DeltaSeconds (Variables|Default|GetTimer))))
      (if (> _output_get (Variables|Default|GetTimeToIgnition))
        (Variables|Default|SetTimer 0.0)
        (for _array_element (Variables|Default|GetPositionsToExpand)
          (Utilities|FlowControl|Sequence
            (:then_0
              (CallFunction|SpawnInstance (+ _array_element "80.000000,46.000000, 0")))
            (:then_1
              (CallFunction|SpawnInstance (+ _array_element "-80.000000,46.000000,0.000000")))
            (:then_2
              (CallFunction|SpawnInstance (+ _array_element "-80.000000,-46.000000, 0")))
            (:then_3
              (CallFunction|SpawnInstance (+ _array_element "80.000000,-46.000000, 0")))
            (:then_4
              (CallFunction|SpawnInstance (+ _array_element "0.000000,92.000000, 0")))
            (:then_5
              (CallFunction|SpawnInstance (+ _array_element "0.000000,-92.000000, 0")))))
        (Utilities|Array|Clear (Variables|Default|GetPositionsToExpand))
        (for _array_element_2 (Variables|Default|GetTMPPositions)
          (Utilities|Array|Add (Variables|Default|GetTotalPositions) _array_element_2)
          (Utilities|Array|Add (Variables|Default|GetPositionsToExpand) _array_element_2))
        (Utilities|Array|Clear (Variables|Default|GetTMPPositions))))))

(fn ConstructionScript)

(fn CheckBounds
  (params (Position :type Vector))
  (bind (_x _y) (Math|Vector|BreakVector Position))
  (return (Math|Boolean|ANDBoolean (< _x 9.6e+02) (> _x -9.6e+02) (< _y 1e+03) (> _y -1e+03))))

(fn SpawnInstance
  (params (Position :type Vector))
  (bind _returnvalue (Transformation|GetActorTransform))
  (bind (_x _y _z) (Math|Vector|BreakVector Position))
  (bind _returnvalue_2 (Transformation|GetActorTransform))
  (bind (_location _rotation _scale) (Math|Transform|BreakTransform _returnvalue))
  (bind (_location_2 _rotation_2 _scale_2) (Math|Transform|BreakTransform _returnvalue_2))
  (if (CallFunction|CheckBounds Position)
    (if (not (Utilities|Array|ContainsItem (Variables|Default|GetTMPPositions) Position))
      (if (not (Utilities|Array|ContainsItem (Variables|Default|GetPositionsToExpand) Position))
        (if (not (Utilities|Array|ContainsItem (Variables|Default|GetTotalPositions) Position))
          (Class|InstancedStaticMeshComponent|AddInstanceWorldSpace (Variables|Default|GetHexagons) (Math|Transform|MakeTransform Position _rotation _scale))
          (Utilities|Array|Add (Variables|Default|GetTMPPositions) Position)
          (Class|InstancedStaticMeshComponent|AddInstanceWorldSpace (Variables|Default|GetFireSymbole) (Math|Transform|MakeTransform (Math|Vector|MakeVector _x _y (+ _z 25.0)) _rotation_2 (* _scale_2 2))))))))