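; HoloWall is a Blueprint for a holographic wall built from three part components that can be switched on or off.
; ShowWall makes all three parts visible and enables query and physics collision, so the wall blocks.
; HideWall hides them and disables their collision.
; The Blueprint only exposes these two events, with no logic of its own to decide when they fire.
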(event Custom|ShowWall
  (bind _wallpart02 (Variables|Default|GetWallPart02))
  (bind _wallpart00 (Variables|Default|GetWallPart00))
  (bind _wallpart01 (Variables|Default|GetWallPart01))
  (Rendering|SetVisibility _wallpart00 true false)
  (Collision|SetCollisionEnabled _wallpart00 "QueryAndPhysics")
  (Rendering|SetVisibility _wallpart01 true false)
  (Collision|SetCollisionEnabled _wallpart01 "QueryAndPhysics")
  (Rendering|SetVisibility _wallpart02 true false)
  (Collision|SetCollisionEnabled _wallpart02 "QueryAndPhysics"))

(event Custom|HideWall
  (bind _wallpart00 (Variables|Default|GetWallPart00))
  (bind _wallpart01 (Variables|Default|GetWallPart01))
  (bind _wallpart02 (Variables|Default|GetWallPart02))
  (Rendering|SetVisibility _wallpart00 false false)
  (Collision|SetCollisionEnabled _wallpart00 "NoCollision")
  (Rendering|SetVisibility _wallpart01 false false)
  (Collision|SetCollisionEnabled _wallpart01 "NoCollision")
  (Rendering|SetVisibility _wallpart02 false false)
  (Collision|SetCollisionEnabled _wallpart02 "NoCollision"))

(fn ConstructionScript)