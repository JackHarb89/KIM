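; Room 1 door control panel that opens once all screws are gone and takes a battery to unlock the door.
; Activation checks for remaining Screw actors, then either plays locked dialogue or enables Tick to swing the plate open by yaw interpolation, disabling Tick near the target.
; Battery placement runs once, revealing the battery, clearing interaction UI state, unlocking the first Door found and turning DoorLight-tagged lights green as temporary feedback.
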(event EventBeginPlay
  (Variables|Default|SetOrginalRotation (Transformation|GetWorldRotation (Variables|Default|GetPlate))))

(event EventTick
  (params (DeltaSeconds :type Float%20%28single-precision%29))
  (bind _dooropenspeed (Variables|Default|GetDoorOpenSpeed))
  (bind _orginalrotation (Variables|Default|GetOrginalRotation))
  (bind _plate (Variables|Default|GetPlate))
  (bind _returnvalue (Transformation|GetWorldRotation _plate))
  (bind (_roll _pitch _yaw) (Math|Rotator|BreakRotator _orginalrotation))
  (bind _returnvalue_2 (* DeltaSeconds _dooropenspeed))
  (bind _returnvalue_3 (+ _yaw 1.3e+02))
  (bind _returnvalue_4 (Math|Rotator|MakeRotator _roll _pitch _returnvalue_3))
  (bind _returnvalue_5 (Math|Rotator|Lerp(Rotator) _returnvalue _returnvalue_4 _returnvalue_2 true))
  (if (Variables|Default|GetLerpDoorOpening)
    (Transformation|SetWorldRotation _plate _returnvalue_5 false false)
    (if (Math|Rotator|Equal(Rotator) _returnvalue_5 _returnvalue_4 5.0)
      (Variables|Default|SetLerpDoorOpening false)
      (Variables|Default|SetIsDoorControlOpen true)
      (Actor|Tick|SetActorTickEnabled false))))

(event EventActivated
  (params (Component :type Primitive%20Component%20Object%20Reference))
  (if (not (Variables|Default|GetIsDoorControlOpen))
    (bind _outactors (Actor|GetAllActorsOfClass "/Game/Blueprint/Room1/Screw.Screw_C"))
    (if (== (Utilities|Array|Length _outactors) 0)
      (Variables|Default|SetLerpDoorOpening true)
      (Actor|Tick|SetActorTickEnabled true)
      (Class|KIMInteractionActor|GetInteractionDialogue "OnOpen")
      (else
        (Class|KIMInteractionActor|GetInteractionDialogue "Press_Locked")))))

(event EventPlacedBattery
  (Utilities|FlowControl|DoOnce false
    (:Completed
      (Development|SetHiddeninGame (Variables|Default|GetBattery) false false)
      (bind _askimhud_bp (Utilities|Casting|CastToKIMHUD_BP (HUD|GetHUD (Game|GetPlayerController 0))))
      (bind _asinteraction_ui (Utilities|Casting|CastToInteractionUI (Variables|/Game/Blueprint/UI/KIMHUD_BP.KIMHUD_BP_C|GetInteractionUI _askimhud_bp)))
      (Default|ClearStateUI _asinteraction_ui)
      (bind _outactors (Actor|GetAllActorsOfClass "/Game/Blueprint/Room1/Door.Door_C"))
      (bind _array_element (Utilities|Array|ForEachLoopwithBreak _outactors :!label _label)
        (:LoopBody
          (Variables|/Game/Blueprint/Room1/Door.Door_C|SetIsLocked _array_element false)
          (goto _label Break))
        (:Completed
          (Class|KIMInteractionActor|GetInteractionDialogue "Place_Battery")
          ;[1 0.03269 0] DoorFeedback Can be removed, just temp
          (bind _outactors_2 (Actor|GetAllActorsOfClass "/Script/Engine.PointLight"))
          (for _array_element_2 _outactors_2
            (if (Components|ComponentHasTag (Variables|/Script/Engine.Light|GetLightComponent _array_element_2) "DoorLight")
              (Rendering|Components|Light|SetLightColor (Variables|/Script/Engine.Light|GetLightComponent _array_element_2) "(R=0.013151,G=0.675000,B=0.000000,A=1.000000)" true))))))))

(fn ConstructionScript)