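; Two-door interactive locker in Room1, with a lockable right door and a one-time video reveal behind the left door's interaction.
; Activated uses component tags to pick the door: left toggles freely and first plays Kim's video, sound and dialogue.
; While locked, right only unlocks if the player holds the item named "Screwdriver", with dialogue either way; later activations toggle it.
; Tick eases each door between closed and swung-open yaw until within tolerance.
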(event EventActivated
  (params (Component :type Primitive%20Component%20Object%20Reference))
  (if (Components|ComponentHasTag Component "Left")
    (Utilities|FlowControl|Sequence
      (:then_0
        (Variables|Default|SetLeftDoorOpen (not (Variables|Default|GetLeftDoorOpen)))
        (Variables|Default|SetLeftDoorLerping true))
      (:then_1
        (Utilities|FlowControl|DoOnce false
          (:Completed
            (Media|MediaPlayer|Play (Variables|Default|GetKimVideo) :!class /Script/MediaAssets.MediaPlayer)
            (Audio|Components|Audio|Play (Variables|Default|GetKimVideoSound) 0.0)
            (Class|KIMInteractionActor|GetInteractionDialogue "Open_Kimberly")))))
    (elif (Components|ComponentHasTag Component "Right")
      (if (Variables|Default|GetIsLocked)
        (bind _ascharacter_bp (Utilities|Casting|CastToCharacter_BP (Game|GetPlayerCharacter 0)))
        (if (Utilities|Enum|Equal(Enum) (Utilities|GetDisplayName (Variables|/Script/KIM.KIMCharacter|GetPickedUpItem _ascharacter_bp)) "Screwdriver")
          (Variables|Default|SetIsLocked false)
          (Class|KIMInteractionActor|GetInteractionDialogue "Unlocked_Thomas")
          (else
            (Class|KIMInteractionActor|GetInteractionDialogue "Press_Thomas_Locked")))
        (else
          (Variables|Default|SetRightDoorOpen (not (Variables|Default|GetRightDoorOpen)))
          (Variables|Default|SetRightDoorLerping true))))))

(event EventBeginPlay
  (Variables|Default|SetLeftOriginalRotation (Transformation|GetWorldRotation (Variables|Default|GetDoorLeft)))
  (Variables|Default|SetRightOriginalRotation (Transformation|GetWorldRotation (Variables|Default|GetDoorRight))))

(event EventTick
  (params (DeltaSeconds :type Float%20%28single-precision%29))
  (bind _rightoriginalrotation (Variables|Default|GetRightOriginalRotation))
  (bind _doorleft (Variables|Default|GetDoorLeft))
  (bind _leftoriginalrotation (Variables|Default|GetLeftOriginalRotation))
  (bind _doorleft_2 (Variables|Default|GetDoorLeft))
  (bind _doorright (Variables|Default|GetDoorRight))
  (bind _doorright_2 (Variables|Default|GetDoorRight))
  (bind _returnvalue (Transformation|GetWorldRotation _doorright))
  (bind (_roll _pitch _yaw) (Math|Rotator|BreakRotator _rightoriginalrotation))
  (bind (_roll_2 _pitch_2 _yaw_2) (Math|Rotator|BreakRotator _leftoriginalrotation))
  (bind _returnvalue_2 (Transformation|GetWorldRotation _doorleft_2))
  (bind _returnvalue_3 (Math|Rotator|Lerp(Rotator) _returnvalue _rightoriginalrotation DeltaSeconds true))
  (bind _returnvalue_4 (Math|Rotator|Lerp(Rotator) _returnvalue_2 _leftoriginalrotation DeltaSeconds true))
  (bind _returnvalue_5 (+ _yaw -1.1e+02))
  (bind _returnvalue_6 (+ _yaw_2 1.1e+02))
  (bind _returnvalue_7 (Math|Rotator|MakeRotator _roll _pitch _returnvalue_5))
  (bind _returnvalue_8 (Math|Rotator|MakeRotator _roll_2 _pitch_2 _returnvalue_6))
  (bind _returnvalue_9 (Math|Rotator|Lerp(Rotator) _returnvalue _returnvalue_7 DeltaSeconds true))
  (bind _returnvalue_10 (Math|Rotator|Lerp(Rotator) _returnvalue_2 _returnvalue_8 DeltaSeconds true))
  (Utilities|FlowControl|Sequence
    (:then_0
      (if (Variables|Default|GetLeftDoorLerping)
        (if (Variables|Default|GetLeftDoorOpen)
          (Transformation|SetWorldRotation _doorleft _returnvalue_10 false false)
          (if (Math|Rotator|Equal(Rotator) _returnvalue_8 _returnvalue_10 1.0)
            (Variables|Default|SetLeftDoorLerping false :!label _label))
          (else
            (Transformation|SetWorldRotation _doorleft _returnvalue_4 false false)
            (if (Math|Rotator|Equal(Rotator) _returnvalue_4 (Variables|Default|GetLeftOriginalRotation) 1.0)
              (goto _label))))))
    (:then_1
      (if (Variables|Default|GetRightDoorLerping)
        (if (Variables|Default|GetRightDoorOpen)
          (Transformation|SetWorldRotation _doorright_2 _returnvalue_9 false false)
          (if (Math|Rotator|Equal(Rotator) _returnvalue_7 _returnvalue_9 1.0)
            (Variables|Default|SetRightDoorLerping false :!label _label_2))
          (else
            (Transformation|SetWorldRotation _doorright_2 _returnvalue_3 false false)
            (if (Math|Rotator|Equal(Rotator) _returnvalue_3 (Variables|Default|GetRightOriginalRotation) 1.0)
              (goto _label_2))))))))

(fn ConstructionScript)