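; Explosive barrel for Room 1 that blows up on contact with fire and can trigger a player failure at the water tank.
; Overlapping an actor tagged Fire calls Explode, which spawns an enlarged explosion emitter and destroys the barrel.
; FireReachedWaterTank searches TriggerBoxes tagged WaterTank; if the barrel overlaps one, it explodes and passes a sarcastic failure message to the player's Character_BP.
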(event Custom|FireReachedWaterTank
  (bind _outactors (Actor|GetAllActorsOfClass 0 "/Script/Engine.TriggerBox"))
  (bind _array_element (Utilities|Array|ForEachLoopwithBreak _outactors)
    (:LoopBody
      (if (Actor|ActorHasTag _array_element "WaterTank")
        (if (Collision|IsOverlappingActor _array_element :!class /Script/Engine.Actor)
          (CallFunction|Explode)
          (bind _ascharacter_bp (Utilities|Casting|CastToCharacter_BP (Game|GetPlayerCharacter 0)))
          (Default|FailedWaterTank _ascharacter_bp "Wow. You are the first one blowing up the whole station! Congratulation..."))))))

(event Custom|Explode
  (bind _returnvalue (Effects|SpawnEmitteratLocation 0 "/Game/VFX/Particles/P_Explosion.P_Explosion" (Transformation|GetActorLocation)))
  (Transformation|SetWorldScale3D _returnvalue "5.000000,5.000000,5.000000")
  (Actor|DestroyActor))

(event Collision|EventActorBeginOverlap
  (params (OtherActor :type Actor%20Object%20Reference))
  (if (Actor|ActorHasTag OtherActor "Fire")
    (CallFunction|Explode)))

(fn ConstructionScript
  (|CallParentFunction))