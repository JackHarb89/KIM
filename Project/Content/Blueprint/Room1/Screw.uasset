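; Interactable screw actor for Room1 that spins and backs out when activated, then destroys itself.
; Activation enables tick and requests the "Screw" interaction dialogue.
; Each tick reapplies the rotation cached at BeginPlay plus accumulated local pitch, while easing the screw slightly along world negative X with a delta-time lerp.
; Once the accumulated rotation passes a full turn, the actor is destroyed.
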(event EventBeginPlay
  (Variables|Default|SetOriginalTransform (Transformation|GetWorldTransform (Variables|Default|GetScrew))))

(event EventTick
  (params (DeltaSeconds :type Float%20%28single-precision%29))
  (bind _originaltransform (Variables|Default|GetOriginalTransform))
  (bind _screw (Variables|Default|GetScrew))
  (bind _location (Math|Transform|BreakTransform _originaltransform))
  (bind (_x _y _z) (Math|Vector|BreakVector _location))
  (if (Variables|Default|GetLerpOutRotation)
    (bind _output_get (Variables|Default|SetTotalRotation (+ (* DeltaSeconds (Variables|Default|GetScrewSpeed)) (Variables|Default|GetTotalRotation))))
    (Transformation|SetWorldRotation _screw (.Rotation (Math|Transform|BreakTransform (Variables|Default|GetOriginalTransform))) false false)
    (Transformation|AddRelativeRotation _screw (Math|Rotator|MakeRotator 0.0 _output_get 0.0) false false)
    (Transformation|SetWorldLocation _screw (Math|Vector|Lerp(Vector) (Transformation|GetWorldLocation _screw) (Math|Vector|MakeVector (+ _x -2.0) _y _z) DeltaSeconds) false false)
    (if (> (Variables|Default|GetTotalRotation) 3.6e+02)
      (Variables|Default|SetLerpOutRotation false)
      (Actor|DestroyActor))))

(event EventActivated
  (params (Component :type Primitive%20Component%20Object%20Reference))
  (Variables|Default|SetLerpOutRotation true)
  (Actor|Tick|SetActorTickEnabled true)
  (Class|KIMInteractionActor|GetInteractionDialogue "Screw"))

(fn ConstructionScript)