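; Interactable ghettoblaster prop in Room 1 whose plate opens to give access to a battery.
; The first activation stores the plate's rotation and starts a Tick-driven LerpRotator that eases it open by a roll offset until within tolerance.
; Activations after that hide the battery and show the battery UI through the HUD's InteractionUI.
; Both steps trigger interaction dialogue, and activations during the opening motion are ignored.
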(event EventTick
  (params (DeltaSeconds :type Float%20%28single-precision%29))
  (bind _plate (Variables|Default|GetPlate))
  (bind _plateoriginalrotation (Variables|Default|GetPlateOriginalRotation))
  (bind _plateopenspeed (Variables|Default|GetPlateOpenSpeed))
  (bind _returnvalue (Transformation|GetWorldRotation _plate))
  (bind (_roll _pitch _yaw) (Math|Rotator|BreakRotator _plateoriginalrotation))
  (bind _returnvalue_2 (* DeltaSeconds _plateopenspeed))
  (bind _returnvalue_3 (- _roll 145.0))
  (bind _returnvalue_4 (Math|Rotator|MakeRotator _returnvalue_3 _pitch _yaw))
  (bind _returnvalue_5 (Math|Rotator|Lerp(Rotator) _returnvalue _returnvalue_4 _returnvalue_2 true))
  (if (Variables|Default|GetPlateRotationActive)
    (Transformation|SetWorldRotation _plate _returnvalue_5 false false)
    (if (Math|Rotator|Equal(Rotator) _returnvalue_5 _returnvalue_4 1.0)
      (Variables|Default|SetPlateRotationActive false)
      (Variables|Default|SetInteractionFinished true))))

(event EventActivated
  (params (Component :type Primitive%20Component%20Object%20Reference))
  (if (not (Variables|Default|GetPlateRotationActive))
    (if (Variables|Default|GetInteractionFinished)
      (Development|SetHiddeninGame (Variables|Default|GetBattery) true false)
      (bind _askimhud_bp (Utilities|Casting|CastToKIMHUD_BP (HUD|GetHUD (Game|GetPlayerController 0))))
      (bind _asinteraction_ui (Utilities|Casting|CastToInteractionUI (Variables|/Game/Blueprint/UI/KIMHUD_BP.KIMHUD_BP_C|GetInteractionUI _askimhud_bp)))
      (Default|ShowBatteryUI _asinteraction_ui)
      (Class|KIMInteractionActor|GetInteractionDialogue "Battery")
      (else
        (Variables|Default|SetPlateOriginalRotation (Transformation|GetWorldRotation (Variables|Default|GetPlate)))
        (Variables|Default|SetPlateRotationActive true)
        (Class|KIMInteractionActor|GetInteractionDialogue "OpenPlate")))))

(fn ConstructionScript)