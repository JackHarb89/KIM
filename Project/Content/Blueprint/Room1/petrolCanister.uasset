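; Room 1 petrol canister item that shows dialogue on pickup and explodes when it overlaps an actor tagged Fire.
; FireReachedWaterTank explodes it if it overlaps a WaterTank-tagged trigger box, then calls the player character's failed-water-tank response after a delay.
; Explode spawns an emitter, plays the explosion component, hides the mesh and destroys the actor shortly after.
; Dialogue lines display through the KIMHUD_BP dialogue widget.
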(event Custom|FireReachedWaterTank
  (bind _outactors (Actor|GetAllActorsOfClass 0 "/Script/Engine.TriggerBox"))
  (bind _array_element (Utilities|Array|ForEachLoopwithBreak _outactors)
    (:LoopBody
      (if (Actor|ActorHasTag _array_element "WaterTank")
        (if (Collision|IsOverlappingActor _array_element :!class /Script/Engine.Actor)
          (CallFunction|Explode)
          (bind _askimhud_bp (Utilities|Casting|CastToKIMHUD_BP (HUD|GetHUD (Game|GetPlayerController 0))))
          (bind _asdialogue (Utilities|Casting|CastToDialogue (Variables|/Game/Blueprint/UI/KIMHUD_BP.KIMHUD_BP_C|GetDialogueUI _askimhud_bp)))
          (Default|SetDialogueText _asdialogue "Yeah feed the fire. Good Idea..." 0 3.0)
          (Utilities|FlowControl|Delay 0 3.0)
          (bind _ascharacter_bp (Utilities|Casting|CastToCharacter_BP (Game|GetPlayerCharacter 0)))
          (Default|FailedWaterTank _ascharacter_bp "How shall a petrol canister blow up a watertank?"))))))

(event Custom|Explode
  (Effects|SpawnEmitteratLocation 0 "/Game/VFX/Particles/P_Explosion.P_Explosion" (Transformation|GetActorLocation))
  (Audio|Components|Audio|Play (Variables|Default|GetExplosion) 0.0)
  (Rendering|SetVisibility (Variables|Default|GetStaticMesh) false false)
  (Utilities|FlowControl|Delay 3.0)
  (Actor|DestroyActor))

(event Collision|EventActorBeginOverlap
  (params (OtherActor :type Actor%20Object%20Reference))
  (if (Actor|ActorHasTag OtherActor "Fire")
    (CallFunction|Explode)
    (bind _askimhud_bp (Utilities|Casting|CastToKIMHUD_BP (HUD|GetHUD (Game|GetPlayerController 0))))
    (bind _asdialogue (Utilities|Casting|CastToDialogue (Variables|/Game/Blueprint/UI/KIMHUD_BP.KIMHUD_BP_C|GetDialogueUI _askimhud_bp)))
    (Default|SetDialogueText _asdialogue "Yeah feed the fire. Good Idea..." 0 3.0)))

(event EventPickUpBP
  (Class|KIMInteractionActor|GetInteractionDialogue "PickUp"))

(event EventStartDialogue
  (params (Dialogue :type Name) (AudioWave :type Sound%20Wave%20Object%20Reference))
  (bind _askimhud_bp (Utilities|Casting|CastToKIMHUD_BP (HUD|GetHUD (Game|GetPlayerController 0))))
  (bind _asdialogue (Utilities|Casting|CastToDialogue (Variables|/Game/Blueprint/UI/KIMHUD_BP.KIMHUD_BP_C|GetDialogueUI _askimhud_bp)))
  (Default|SetDialogueText _asdialogue Dialogue 0 3.0))

(fn ConstructionScript
  (|CallParentFunction))