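; Interactable sliding door that, when activated, plays locked or unlocked dialogue and opens only if unlocked.
; It records the closed positions of its upper and lower parts at BeginPlay, then Tick eases them apart vertically with a delta-time-scaled lerp from their current locations.
; Once the lower part nearly stops moving, it disables Tick and clears its interaction type, with no closing logic.
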(event EventTick
  (params (DeltaSeconds :type Float%20%28single-precision%29))
  (bind _lowerdoorpart (Variables|Default|GetLowerDoorPart))
  (bind _dooropenspeed (Variables|Default|GetDoorOpenSpeed))
  (bind _lowerdoorclosedlocation (Variables|Default|GetLowerDoorClosedLocation))
  (bind _upperdoorpart (Variables|Default|GetUpperDoorPart))
  (bind _returnvalue (Transformation|GetWorldLocation _lowerdoorpart))
  (bind _returnvalue_2 (+ _lowerdoorclosedlocation "0, 0,-110.000000"))
  (bind _returnvalue_3 (* DeltaSeconds _dooropenspeed))
  (bind _returnvalue_4 (Math|Vector|Lerp(Vector) _returnvalue _returnvalue_2 _returnvalue_3))
  (if (Variables|Default|GetIsLerping)
    (Utilities|FlowControl|Sequence
      (:then_0
        (Transformation|SetWorldLocation _upperdoorpart (Math|Vector|Lerp(Vector) (Transformation|GetWorldLocation _upperdoorpart) (+ (Variables|Default|GetUpperDoorClosedLocation) "0, 0,110.000000") _returnvalue_3) false false))
      (:then_1
        (Transformation|SetWorldLocation _lowerdoorpart _returnvalue_4 false false)
        (if (Math|Vector|Equal(Vector) _returnvalue _returnvalue_4 0.05)
          (Actor|Tick|SetActorTickEnabled false)
          (Variables|Default|SetIsLerping false)
          (Variables|Default|SetInteractionType "NONE"))))))

(event EventBeginPlay
  (Variables|Default|SetUpperDoorClosedLocation (Transformation|GetWorldLocation (Variables|Default|GetUpperDoorPart)))
  (Variables|Default|SetLowerDoorClosedLocation (Transformation|GetWorldLocation (Variables|Default|GetLowerDoorPart))))

(event EventActivated
  (params (Component :type Primitive%20Component%20Object%20Reference))
  (if (Variables|Default|GetIsLocked)
    (Class|KIMInteractionActor|GetInteractionDialogue "Press_Locked")
    (else
      (Actor|Tick|SetActorTickEnabled true)
      (Variables|Default|SetIsLerping true)
      (Class|KIMInteractionActor|GetInteractionDialogue "Press_Unlocked"))))

(fn ConstructionScript)