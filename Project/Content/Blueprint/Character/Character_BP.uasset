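; Player character Blueprint that adds walking head bob and links the player to the KIM HUD and the energy puzzle.
; Holding W plays a timeline that offsets the camera vertically, and releasing it eases back, unless in rotation state.
; Escape or H closes the active puzzle; solving it hides the UI, disables the first EnergyConsole and starts all Sprinklers.
; E toggles the eye-opening animation for debugging, and an opening dialogue sequence sits unconnected.
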(event Custom|SolvedEnergyPuzzle
  (bind _returnvalue (Game|GetPlayerController 0))
  (Utilities|FlowControl|Sequence
    (:then_0
      (Utilities|FlowControl|Delay 0 1.0)
      (bind _askimhud_bp (Utilities|Casting|CastToKIMHUD_BP (HUD|GetHUD _returnvalue)))
      (Widget|SetVisibility (Variables|/Game/Blueprint/UI/KIMHUD_BP.KIMHUD_BP_C|GetEnergyPuzzle _askimhud_bp) "Hidden")
      (Variables|Default|SetEnergyPuzzleActive false)
      (Variables|/Script/Engine.PlayerController|SetbShowMouseCursor _returnvalue false)
      (Development|PrintString 0 "SUCCESS!!!!")
      (bind _outactors (Actor|GetAllActorsOfClass 0 "/Game/Blueprint/EnergyConsole.EnergyConsole_C"))
      (bind _array_element (Utilities|Array|ForEachLoopwithBreak _outactors :!label _label)
        (:LoopBody
          (Variables|/Script/KIM.KIMInteractionActor|SetInteractionType _array_element "NONE")
          (goto _label Break))))
    (:then_1
      (bind _outactors_2 (Actor|GetAllActorsOfClass "/Game/Blueprint/sprinkler.Sprinkler_C"))
      (for _array_element_2 _outactors_2
        (Default|StartH20 _array_element_2)))))

(event EventBeginPlay
  (bind _cameracomponent (Variables|Default|GetCameraComponent))
  (bind _returnvalue (Transformation|GetRelativeTransform _cameracomponent))
  (bind (_location _rotation) (Math|Transform|BreakTransform _returnvalue))
  (Variables|Default|SetOriginalRelativeCameraLocation _location)
  (Variables|Default|SetOriginalRelativeCameraRotation _rotation))

(event EventSwitchIconState
  (params (Type :type EKIMInteractionTypes%20Enum :default "NONE"))
  (bind _askimhud_bp (Utilities|Casting|CastToKIMHUD_BP (HUD|GetHUD (Game|GetPlayerController 0))))
  (Default|SwitchIconState _askimhud_bp Type))

(event Input|KeyboardEvents|E
  (params (Key :type Key%20Structure :default "AnyKey"))
  ;[1 1 1] Debug
  (:Pressed
    (bind _askimhud_bp (Utilities|Casting|CastToKIMHUD_BP (HUD|GetHUD (Game|GetPlayerController 0))))
    (bind _aseys_opening (Utilities|Casting|CastToEysOpening (Variables|/Game/Blueprint/UI/KIMHUD_BP.KIMHUD_BP_C|GetEyeUI _askimhud_bp)))
    (Default|ToggleAnimation _aseys_opening)))

(event Input|KeyboardEvents|W
  (params (Key :type Key%20Structure :default "AnyKey"))
  ;[1 1 1] Bobcycle
  (:Released
    (if (not (Variables|Default|GetIsInRoationState))
      (bind _headbob_loop (Timeline|BobcycleEnd PlayFromStart)
        (:Update
          (Transformation|SetRelativeLocation (Variables|Default|GetCameraComponent) (Math|Vector|Lerp(Vector) (Variables|/Script/Engine.SceneComponent|GetRelativeLocation (Variables|Default|GetCameraComponent)) (Variables|Default|GetOriginalRelativeCameraLocation) _headbob_loop) false false))))))

(event Input|KeyboardEvents|Escape
  (params (Key :type Key%20Structure :default "AnyKey"))
  (bind _returnvalue (Game|GetPlayerController 0))
  (:Pressed
    (if (Variables|Default|GetEnergyPuzzleActive)
      (bind _askimhud_bp (Utilities|Casting|CastToKIMHUD_BP (HUD|GetHUD _returnvalue)))
      (Widget|SetVisibility (Variables|/Game/Blueprint/UI/KIMHUD_BP.KIMHUD_BP_C|GetEnergyPuzzle _askimhud_bp) "Hidden")
      (Variables|Default|SetEnergyPuzzleActive false)
      (Variables|/Script/Engine.PlayerController|SetbShowMouseCursor _returnvalue false))))

(event Input|KeyboardEvents|H
  (params (Key :type Key%20Structure :default "AnyKey"))
  (bind _returnvalue (Game|GetPlayerController 0))
  (:Pressed
    (if (Variables|Default|GetEnergyPuzzleActive)
      (bind _askimhud_bp (Utilities|Casting|CastToKIMHUD_BP (HUD|GetHUD _returnvalue)))
      (Widget|SetVisibility (Variables|/Game/Blueprint/UI/KIMHUD_BP.KIMHUD_BP_C|GetEnergyPuzzle _askimhud_bp) "Hidden")
      (Variables|Default|SetEnergyPuzzleActive false)
      (Variables|/Script/Engine.PlayerController|SetbShowMouseCursor _returnvalue false))))

(event Input|KeyboardEvents|W
  (params (Key :type Key%20Structure :default "AnyKey"))
  (bind _isinroationstate (Variables|Default|GetIsInRoationState))
  (bind _originalrelativecameralocation (Variables|Default|GetOriginalRelativeCameraLocation))
  ;[1 1 1] Bobcycle
  (:Pressed
    (if (not _isinroationstate)
      (bind _headbob_loop (Timeline|bobcycle Play)
        (:Update
          (Transformation|SetRelativeLocation (Variables|Default|GetCameraComponent) (Math|Vector|Lerp(Vector) _originalrelativecameralocation (+ _originalrelativecameralocation (* (Math|Vector|MakeVector 0.0 0.0 1.0) (Variables|Default|GetShakeIntensity))) _headbob_loop) false false)))))
  (:Released
    (if (not _isinroationstate)
      (Timeline|bobcycle Stop))))

(fn ConstructionScript)