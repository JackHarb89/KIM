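; Physics interaction object that the player can pick up, drop and throw, with support for voiced dialogue.
; Pickup disables mesh physics and plays an interaction sound, while dropping and throwing re-enable physics.
; Throws apply a velocity-change impulse along the player capsule's forward vector, reduced by the object's Weight.
; StartDialogue assigns the audio wave and passes text, audio component and clip duration to the HUD's dialogue widget.
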(event EventThrown
  (params (Intensity :type Float%20%28single-precision%29))
  (bind _staticmesh (Variables|Default|GetStaticMesh))
  (Physics|SetSimulatePhysics _staticmesh true)
  (Physics|AddImpulse _staticmesh (* (Math|Vector|GetForwardVector (Variables|/Script/Engine.Character|GetCapsuleComponent (Game|GetPlayerCharacter 0))) (- Intensity (* (Variables|Default|GetWeight) 1e+01))) "None" true))

(event EventPickedUp
  (Physics|SetSimulatePhysics (Variables|Default|GetStaticMesh) false)
  (Audio|Components|Audio|Play (Variables|Default|GetInteractionSound) 0.0))

(event EventDroped
  (Physics|SetSimulatePhysics (Variables|Default|GetStaticMesh) true))

(event EventStartDialogue
  (params (Dialogue :type Name) (AudioWave :type Sound%20Wave%20Object%20Reference))
  (bind _askimhud_bp (Utilities|Casting|CastToKIMHUD_BP (HUD|GetHUD (Game|GetPlayerController 0))))
  (bind _asdialogue (Utilities|Casting|CastToDialogue (Variables|/Game/Blueprint/UI/KIMHUD_BP.KIMHUD_BP_C|GetDialogueUI _askimhud_bp)))
  (Audio|Components|Audio|SetSound (Variables|Default|GetDialogue) AudioWave)
  (if (Utilities|IsValid AudioWave)
    (Default|SetDialogueText _asdialogue Dialogue (Variables|Default|GetDialogue) (Variables|/Script/Engine.SoundBase|GetDuration AudioWave))))

(fn ConstructionScript)