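; Alarm light actor for the presentation room that pulses a point light's intensity until switched to normal lighting.
; While AllowLerping is set, Tick eases intensity toward a peak or zero, flipping LerpOn when within tolerance of the target.
; The NormalMode event stops the pulsing and sets a steady, brighter, pale-yellow light.
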(event Custom|NormalMode
  (bind _pointlight (Variables|Default|GetPointLight))
  (Variables|Default|SetAllowLerping false)
  (Rendering|Components|Light|SetLightColor _pointlight "(R=1.000000,G=0.995317,B=0.708452,A=1.000000)" true)
  (Rendering|Components|Light|SetIntensity _pointlight 4e+03))

(event EventBeginPlay)

(event EventActorBeginOverlap
  (params (OtherActor :type Actor%20Object%20Reference)))

(event EventTick
  (params (DeltaSeconds :type Float%20%28single-precision%29))
  (bind _returnvalue (* 2 DeltaSeconds))
  (bind _pointlight (Variables|Default|GetPointLight))
  (bind _intensity (Variables|/Script/Engine.LightComponentBase|GetIntensity _pointlight))
  (bind _returnvalue_2 (Math|Float|Lerp _intensity 0.0 _returnvalue))
  (bind _returnvalue_3 (Math|Float|Lerp _intensity 2.5e+03 _returnvalue))
  (if (Variables|Default|GetAllowLerping)
    (if (Variables|Default|GetLerpOn)
      (Rendering|Components|Light|SetIntensity _pointlight _returnvalue_3)
      (if (Math|Float|NearlyEqual(Float) _returnvalue_3 2.5e+03 5e+01)
        (Variables|Default|SetLerpOn false))
      (else
        (Rendering|Components|Light|SetIntensity _pointlight _returnvalue_2)
        (if (Math|Float|NearlyEqual(Float) _returnvalue_2 0.0 5e+01)
          (Variables|Default|SetLerpOn true))))))

(fn ConstructionScript)