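; Forward button in the presentation room that drives the Pitch_Screen actors when activated.
; Activated enables Tick, which lerps the button slightly down and back to its original height, then disables itself.
; For every EnergyPort found, it calls ButtonActivated(true) on all screens if that port is powered, otherwise StartKim.
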(event EventActivated
  (params (Component :type Primitive%20Component%20Object%20Reference))
  (Actor|Tick|SetActorTickEnabled true)
  (bind _outactors (Actor|GetAllActorsOfClass "/Game/Blueprint/PresentationRoom/EnergyPort.EnergyPort_C"))
  (for _array_element _outactors
    (if (Variables|/Game/Blueprint/PresentationRoom/EnergyPort.EnergyPort_C|GetIsPowered _array_element)
      (bind _outactors_2 (Actor|GetAllActorsOfClass "/Game/Blueprint/PresentationRoom/Pitch_Screen.Pitch_Screen_C"))
      (for _array_element_2 _outactors_2
        (Default|ButtonActivated _array_element_2 true))
      (else
        (bind _outactors_3 (Actor|GetAllActorsOfClass "/Game/Blueprint/PresentationRoom/Pitch_Screen.Pitch_Screen_C"))
        (for _array_element_3 _outactors_3
          (Default|StartKim _array_element_3))))))

(event EventBeginPlay
  (bind _returnvalue (Transformation|GetActorLocation))
  (bind _z (Math|Vector|BreakVector _returnvalue))
  (Variables|Default|SetOrigin _z)
  (Variables|Default|SetTarget (- _z 2.0)))

(event Collision|EventActorBeginOverlap
  (params (OtherActor :type Actor%20Object%20Reference)))

(event EventTick
  (params (DeltaSeconds :type Float%20%28single-precision%29))
  (bind _returnvalue (Transformation|GetActorLocation))
  (bind _returnvalue_2 (Transformation|GetActorLocation))
  (bind _returnvalue_3 (* DeltaSeconds 4.0))
  (bind _target (Variables|Default|GetTarget))
  (bind _origin (Variables|Default|GetOrigin))
  (bind (_x _y _z) (Math|Vector|BreakVector _returnvalue))
  (bind (_x_2 _y_2 _z_2) (Math|Vector|BreakVector _returnvalue_2))
  (bind _returnvalue_4 (Math|Float|Lerp _z _origin _returnvalue_3))
  (bind _returnvalue_5 (Math|Float|Lerp _z_2 _target _returnvalue_3))
  (if (Variables|Default|GetPressed)
    (Transformation|SetActorLocation (Math|Vector|MakeVector _x _y _returnvalue_4) false false)
    (if (Math|Float|NearlyEqual(Float) _origin _returnvalue_4 0.1)
      (Actor|Tick|SetActorTickEnabled false)
      (Variables|Default|SetPressed false))
    (else
      (Transformation|SetActorLocation (Math|Vector|MakeVector _x_2 _y_2 _returnvalue_5) false false)
      (if (Math|Float|NearlyEqual(Float) _target _returnvalue_5 0.1)
        (Variables|Default|SetPressed true)))))

(fn ConstructionScript)