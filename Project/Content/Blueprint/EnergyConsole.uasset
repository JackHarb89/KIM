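; EnergyConsole is a console Blueprint that opens the energy puzzle UI when it receives its Activated event.
; It checks the player character's EnergyPuzzleActive flag so the puzzle only opens if not already active.
; It then makes the EnergyPuzzle element on KIMHUD_BP visible, sets the flag and shows the mouse cursor.
; Closing the puzzle is not handled here, and the construction script only calls its parent.
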(event EventActivated
  (params (Component :type Primitive%20Component%20Object%20Reference))
  (bind _returnvalue (Game|GetPlayerController 0))
  (bind _ascharacter_bp (Utilities|Casting|CastToCharacter_BP (Game|GetPlayerCharacter 0)))
  (if (not (Variables|/Game/Blueprint/Character/Character_BP.Character_BP_C|GetEnergyPuzzleActive _ascharacter_bp))
    (bind _askimhud_bp (Utilities|Casting|CastToKIMHUD_BP (HUD|GetHUD _returnvalue)))
    (Widget|SetVisibility (Variables|/Game/Blueprint/UI/KIMHUD_BP.KIMHUD_BP_C|GetEnergyPuzzle _askimhud_bp) "Visible")
    (Variables|/Game/Blueprint/Character/Character_BP.Character_BP_C|SetEnergyPuzzleActive _ascharacter_bp true)
    (Variables|/Script/Engine.PlayerController|SetbShowMouseCursor _returnvalue true)))

(fn ConstructionScript
  (|CallParentFunction))