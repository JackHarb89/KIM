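; EnergyCell is an actor for a physics-driven energy cell that can be picked up, dropped and thrown.
; Pickup and drop events switch physics simulation on the Cell component off and on.
; Throwing enables physics and applies a velocity-change impulse along the player capsule's forward vector, with the given intensity reduced by a multiple of Weight.
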(event EventActorBeginOverlap
  (params (OtherActor :type Actor%20Object%20Reference)))

(event EventTick
  (params (DeltaSeconds :type Float%20%28single-precision%29)))

(event EventPickedUp
  (Physics|SetSimulatePhysics (Variables|Default|GetCell) false))

(event EventThrown
  (params (Intensity :type Float%20%28single-precision%29))
  (bind _cell (Variables|Default|GetCell))
  (Physics|SetSimulatePhysics _cell true)
  (Physics|AddImpulse _cell (* (Math|Vector|GetForwardVector (Variables|/Script/Engine.Character|GetCapsuleComponent (Game|GetPlayerCharacter 0))) (- Intensity (* (Variables|Default|GetWeight) 1e+01))) "None" true))

(event EventDroped
  (Physics|SetSimulatePhysics (Variables|Default|GetCell) true))

(event EventBeginPlay)

(fn ConstructionScript)