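; Pitch_Screen is a presentation screen actor that steps through a slide deck by swapping the material on its Screen component.
; StartKim shows the opening video slide and restarts its media and audio.
; ButtonActivated moves the slide index forward or back, undoing steps past either limit, then switches to that slide's material.
; Video slides rewind and play their media, with separate audio components started or stopped on certain slides.
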(event Custom|ButtonActivated
  (params (IsForward :type Boolean))
  (bind _slides (Variables|Default|GetSlides))
  (bind _screen (Variables|Default|GetScreen))
  (bind _9_screen (Variables|Default|Get9_Screen))
  (bind _10_screen (Variables|Default|Get10_Screen))
  (bind _11_screen (Variables|Default|Get11_Screen))
  (if IsForward
    (bind _result (Math|Integer|IncrementInt _slides :!label _label)
      (:%20%20
        (if (> _result (Variables|Default|GetMaxSlides))
          (bind _result_2 (Math|Integer|DecrementInt _slides :!label _label_2)
            (:%20%20
              (if (< _result_2 -1)
                (goto _label)
                (else
                  _)))))))
    (else
      (goto _label_2)))
  (switch int _slides
    (:0
      (Rendering|Material|SetMaterial _screen 0 "/Game/Movies/1_screen_Mat.1_screen_Mat"))
    (:1
      (Rendering|Material|SetMaterial _screen 0 "/Game/Movies/2_screen_Mat.2_screen_Mat"))
    (:2
      (Rendering|Material|SetMaterial _screen 0 "/Game/Movies/3_screen_Mat.3_screen_Mat"))
    (:3
      (Rendering|Material|SetMaterial _screen 0 "/Game/Movies/4_screen_Mat.4_screen_Mat"))
    (:4
      (Rendering|Material|SetMaterial _screen 0 "/Game/Movies/5_screen_Mat.5_screen_Mat"))
    (:5
      (Rendering|Material|SetMaterial _screen 0 "/Game/Movies/6_screen_Mat.6_screen_Mat"))
    (:6
      (Rendering|Material|SetMaterial _screen 0 "/Game/Movies/7_screen_Mat.7_screen_Mat"))
    (:7
      (Rendering|Material|SetMaterial _screen 0 "/Game/Movies/8_screen_Mat.8_screen_Mat"))
    (:8
      (Rendering|Material|SetMaterial _screen 0 "/Game/Movies/9_screen_Tex_Mat.9_screen_Tex_Mat")
      (Class|MediaPlayer|Rewind _9_screen)
      (Media|MediaPlayer|Play _9_screen :!class /Script/MediaAssets.MediaPlayer)
      (Audio|Components|Audio|Stop (Variables|Default|Get10_screen_Wav)))
    (:9
      (Rendering|Material|SetMaterial _screen 0 "/Game/Movies/10_screen_Tex_Mat.10_screen_Tex_Mat")
      (Class|MediaPlayer|Rewind _10_screen)
      (Media|MediaPlayer|Play _10_screen :!class /Script/MediaAssets.MediaPlayer)
      (Audio|Components|Audio|Stop (Variables|Default|Get11_screen_Wav))
      (Audio|Components|Audio|Play (Variables|Default|Get10_screen_Wav) 0.0))
    (:10
      (Rendering|Material|SetMaterial _screen 0 "/Game/Movies/11_screen_Tex_Mat.11_screen_Tex_Mat")
      (Class|MediaPlayer|Rewind _11_screen)
      (Media|MediaPlayer|Play _11_screen :!class /Script/MediaAssets.MediaPlayer)
      (Audio|Components|Audio|Stop (Variables|Default|Get10_screen_Wav))
      (Audio|Components|Audio|Play (Variables|Default|Get11_screen_Wav) 0.0))
    (:11
      (Rendering|Material|SetMaterial _screen 0 "/Game/Movies/12_screen_Mat.12_screen_Mat")
      (Audio|Components|Audio|Stop (Variables|Default|Get0_screen_Wav))
      (Audio|Components|Audio|Stop (Variables|Default|Get10_screen_Wav))
      (Audio|Components|Audio|Stop (Variables|Default|Get11_screen_Wav)))
    (:12
      (Rendering|Material|SetMaterial _screen 0 "/Game/Movies/13_screen_Mat.13_screen_Mat"))))

(event Custom|StartKim
  (bind _0_screen (Variables|Default|Get0_Screen))
  (bind _0_screen_wav (Variables|Default|Get0_screen_Wav))
  (Rendering|Material|SetMaterial (Variables|Default|GetScreen) 0 "/Game/Movies/0_screen_Tex_Mat.0_screen_Tex_Mat")
  (Class|MediaPlayer|Rewind _0_screen)
  (Audio|Components|Audio|Stop _0_screen_wav)
  (Media|MediaPlayer|Play _0_screen :!class /Script/MediaAssets.MediaPlayer)
  (Audio|Components|Audio|Play _0_screen_wav 0.0))

(event EventBeginPlay)

(event EventActorBeginOverlap
  (params (OtherActor :type Actor%20Object%20Reference)))

(event EventTick
  (params (DeltaSeconds :type Float%20%28single-precision%29)))

(fn ConstructionScript)