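; Sliding double door actor that opens when the player character enters its trigger and closes when they leave.
; Overlap events on the Opener component, filtered to Character_BP, play or reverse the Opening timeline.
; The timeline track, scaled by Distance, moves DoorLeft and DoorRight in opposite directions along local X without sweep.
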(event OnComponentBeginOverlap(Opener)
  (params (OtherActor :type Actor%20Object%20Reference) (OtherComp :type Primitive%20Component%20Object%20Reference) (OtherBodyIndex :type Integer) (bFromSweep :type Boolean) (SweepResult :type Hit%20Result%20Structure%20%28by%20ref%29))
  (Utilities|Casting|CastToCharacter_BP OtherActor)
  (bind _newtrack_0 (Timeline|Opening Play)
    (:Update
      (Transformation|SetRelativeLocation (Variables|Default|GetDoor_Left) (Math|Vector|MakeVector (* (* _newtrack_0 (Variables|Default|GetDistance)) -1.0) 0.0 0.0) false false)
      (Transformation|SetRelativeLocation (Variables|Default|GetDoor_Right) (Math|Vector|MakeVector (* _newtrack_0 (Variables|Default|GetDistance)) 0.0 0.0) false false))))

(event OnComponentEndOverlap(Opener)
  (params (OtherActor :type Actor%20Object%20Reference) (OtherComp :type Primitive%20Component%20Object%20Reference) (OtherBodyIndex :type Integer))
  (Utilities|Casting|CastToCharacter_BP OtherActor)
  (bind _newtrack_0 (Timeline|Opening Reverse)
    (:Update
      (Transformation|SetRelativeLocation (Variables|Default|GetDoor_Left) (Math|Vector|MakeVector (* (* _newtrack_0 (Variables|Default|GetDistance)) -1.0) 0.0 0.0) false false)
      (Transformation|SetRelativeLocation (Variables|Default|GetDoor_Right) (Math|Vector|MakeVector (* _newtrack_0 (Variables|Default|GetDistance)) 0.0 0.0) false false))))

(fn ConstructionScript)