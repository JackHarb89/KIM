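; One-shot trigger actor that switches on level sounds the first time any actor begins overlapping it.
; A DoOnce feeds a sequence that finds every Oven, AmbientSound and Vent actor in turn.
; Ovens get StartSound called directly, while ambient and vent audio components play only if SoundOn is set on the KIMGameInstance.
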(event Collision|EventActorBeginOverlap
  (params (OtherActor :type Actor%20Object%20Reference))
  (Utilities|FlowControl|DoOnce false
    (:Completed
      (Utilities|FlowControl|Sequence
        (:then_0
          (bind _outactors (Actor|GetAllActorsOfClass "/Game/Blueprint/Room1/Oven.Oven_C"))
          (for _array_element _outactors
            (Default|StartSound _array_element)))
        (:then_1
          (bind _outactors_2 (Actor|GetAllActorsOfClass "/Script/Engine.AmbientSound"))
          (for _array_element_2 _outactors_2
            (bind _askimgame_instance (Utilities|Casting|CastToKIMGameInstance (Game|GetGameInstance)))
            (if (Variables|/Game/Blueprint/KIMGameInstance.KIMGameInstance_C|GetSoundOn _askimgame_instance)
              (Audio|Components|Audio|Play (Variables|/Script/Engine.AmbientSound|GetAudioComponent _array_element_2) 0.0))))
        (:then_2
          (bind _outactors_3 (Actor|GetAllActorsOfClass "/Game/Blueprint/Room1/Vent.Vent_C"))
          (for _array_element_3 _outactors_3
            (bind _askimgame_instance_2 (Utilities|Casting|CastToKIMGameInstance (Game|GetGameInstance)))
            (if (Variables|/Game/Blueprint/KIMGameInstance.KIMGameInstance_C|GetSoundOn _askimgame_instance_2)
              (Audio|Components|Audio|Play (Variables|/Game/Blueprint/Room1/Vent.Vent_C|GetVentSound _array_element_3) 0.0))))))))

(fn ConstructionScript)